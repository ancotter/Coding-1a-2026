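; BP_Door is a locked door actor that opens only for a player carrying a key.
; On overlap it casts the other actor to BP_ThirdPersonCharacter and checks that character's TotalKeys.
; With a key available, it decrements both TotalKeys and TotalDoors on the character, prints text and destroys itself.
; Without one, it prints that the door is locked.
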(event EventBeginPlay)

(event Collision|EventActorBeginOverlap
  (params (OtherActor :type Actor%20Object%20Reference))
  (bind _asbp_third_person_character (Utilities|Casting|CastToBP_ThirdPersonCharacter OtherActor)) ; is it the player?
  (if (> (Variables|/Game/ThirdPerson/Blueprints/BP_ThirdPersonCharacter.BP_ThirdPersonCharacter_C|GetTotalKeys _asbp_third_person_character) 0)
    (Math|Integer|DecrementInt (Variables|/Game/ThirdPerson/Blueprints/BP_ThirdPersonCharacter.BP_ThirdPersonCharacter_C|GetTotalKeys _asbp_third_person_character)
      (:%20%20
        (Math|Integer|DecrementInt (Variables|/Game/ThirdPerson/Blueprints/BP_ThirdPersonCharacter.BP_ThirdPersonCharacter_C|GetTotalDoors _asbp_third_person_character)
          (:%20%20
            (Development|PrintText "... or you can delete it.")
            (Actor|DestroyActor)))))
    (else
      (Development|PrintText "The Door is Locked"))))

(event EventTick
  (params (DeltaSeconds :type Float%20%28single-precision%29)))

(fn ConstructionScript)