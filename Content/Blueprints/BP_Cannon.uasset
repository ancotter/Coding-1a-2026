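; BP_Cannon is a cannon actor that fires a physics cannonball one second after play begins and again whenever an actor overlaps it.
; Each shot prints a message, spawns the ball at BoxSpawnPoint's transform and pushes its Cube along its forward vector by Force, applied as an acceleration change.
; An unconnected, unfinished branch sketches launching the third-person character instead, casting the overlapping actor and disabling its capsule physics.
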(event Custom|Launch%20Cannonball
  (Development|PrintText "Ka-pow!"))

(event EventBeginPlay
  (Utilities|FlowControl|Delay 1.0)
  (CallFunction|LaunchCannonball)
  (bind _returnvalue (Game|SpawnActorfromClass "/Game/Blueprints/BP_Cannonball.BP_Cannonball_C" (Transformation|GetWorldTransform (Variables|Default|GetBoxSpawnPoint)) "Undefined" "MultiplyWithRoot" 0 0))
  (Physics|AddForce (Variables|/Game/Blueprints/BP_Cannonball.BP_Cannonball_C|GetCube _returnvalue) (* (Math|Vector|GetForwardVector (Variables|/Game/Blueprints/BP_Cannonball.BP_Cannonball_C|GetCube _returnvalue)) (Variables|Default|GetForce)) "None" true))

(event Collision|EventActorBeginOverlap
  (params (OtherActor :type Actor%20Object%20Reference))
  (CallFunction|LaunchCannonball)
  (bind _returnvalue (Game|SpawnActorfromClass "/Game/Blueprints/BP_Cannonball.BP_Cannonball_C" (Transformation|GetWorldTransform (Variables|Default|GetBoxSpawnPoint)) "Undefined" "MultiplyWithRoot" 0 0))
  (Physics|AddForce (Variables|/Game/Blueprints/BP_Cannonball.BP_Cannonball_C|GetCube _returnvalue) (* (Math|Vector|GetForwardVector (Variables|/Game/Blueprints/BP_Cannonball.BP_Cannonball_C|GetCube _returnvalue)) (Variables|Default|GetForce)) "None" true))

(event EventTick
  (params (DeltaSeconds :type Float%20%28single-precision%29)))

(fn ConstructionScript)